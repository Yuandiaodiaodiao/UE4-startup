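; Master building actor that serves as a placement preview, then becomes a constructed building.
; Preview supports 90-degree rotation and resource variants that update ghost color and build widget, hiding both mesh and widget when overlapping built buildings.
; OnBuild applies the resource's material, blocking collision and stats, then a looping timer raises health to maximum over the build time.
; Player-sight events toggle the health bar once built.
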(event `self.ReceiveBeginPlay`
  (bind _buildingmesh (`self.BuildingMesh`))
  (bind _resource (`self.Resource`))
  (bind _returnvalue (`PrimitiveComponent.CreateDynamicMaterialInstance` _buildingmesh 0 (`PrimitiveComponent.GetMaterial` _buildingmesh 0) "None"))
  (set `self.DynamicMaterial` _returnvalue)
  (bind _asw_building_widget (cast `/Game/BuildingSystem/Widgets/W_BuildingWidget` (`WidgetComponent.GetUserWidgetObject` (`self.BuildWidget`))))
  (bind _output_get (set `self.BuildWidgetReference` _asw_building_widget))
  (bind _asw_building_health_bar (cast `/Game/BuildingSystem/Widgets/W_BuildingHealthBar` (`WidgetComponent.GetUserWidgetObject` (`self.HealthBar`))))
  (set `self.HealthBarRef` _asw_building_health_bar)
  (`/Game/BuildingSystem/Widgets/W_BuildingWidget.Update` _output_get (`BlueprintMapLibrary.Map_Find` (`self.ResourceVersions`) _resource) _resource)
  (`/Game/BuildingSystem/Blueprints/Classes/BpC_Building_Stat.InitializeManager` (`self.BpC_Building_Stat`) self)
  (`SceneComponent.SetVisibility` (`self.BuildWidget`) true false))

(event `SetCanBeBuilt`
  (params (`New Value` :type Boolean))
  (bind _output_get (set `self.CanBeBuilt?` `New Value`))
  (`/Game/BuildingSystem/Widgets/W_BuildingWidget.SetCanBeBuilt` (`self.BuildWidgetReference`) _output_get))

(event `OnBuild`
  (params (Resource :type "/Game/BuildingSystem/Blueprints/Classes/ResourceClass/Bp_Master_Resource Class Reference"))
  (bind _bpc_building_stat (`self.BpC_Building_Stat`))
  (bind _buildingmesh (`self.BuildingMesh`))
  (bind (_requiredamount _buildingtime _maximumhealth) (break `/Game/BuildingSystem/Blueprints/Structures/s_Building_Resource_Version` (`BlueprintMapLibrary.Map_Find` (`self.ResourceVersions`) Resource)))
  (if (`KismetSystemLibrary.IsValidClass` Resource)
    (set `self.Built?` true)
    (`PrimitiveComponent.SetCollisionResponseToAllChannels` _buildingmesh "ECR_Block")
    (`PrimitiveComponent.SetMaterial` _buildingmesh 0 (`.BuildingMaterial_12_E9655F684D928BF65F2163B601E5E49C` (break `/Game/BuildingSystem/Blueprints/Structures/s_ResourceData` (defaults `Object` Resource))))
    (`ActorComponent.K2_DestroyComponent` (`self.BuildWidget`))
    (`/Game/BuildingSystem/Blueprints/Classes/BpC_Building_Stat.SetMaxStatValue` _bpc_building_stat "NewEnumerator0" _maximumhealth false)
    (`/Game/BuildingSystem/Blueprints/Classes/BpC_Master_StateManager.SetStat` _bpc_building_stat "NewEnumerator2" 0 true)
    (set `self.BuildingTime` _buildingtime)
    (`/Game/BuildingSystem/Widgets/W_BuildingHealthBar.InitializeBar` (`self.HealthBarRef`) (`/Game/BuildingSystem/Blueprints/Classes/BpC_Building_Stat.GetMaxHealth` _bpc_building_stat))
    (`SceneComponent.SetVisibility` (`self.HealthBar`) true false)
    (bind _returnvalue (`KismetSystemLibrary.K2_SetTimerDelegate` (delegate `BuildingTick`) (`self.InterVal`) true))
    (set `self.BuildingTimerHandle` _returnvalue)
    (`KismetSystemLibrary.Delay` (+ (`self.BuildingTime`) (`self.InterVal`)))
    (`self.OnBuildingEnd`)))

(event `BuildingTick`
  (bind _bpc_building_stat (`self.BpC_Building_Stat`))
  (bind _out (`/Game/BuildingSystem/Blueprints/Classes/BpC_Building_Stat.GetMaxHealth` _bpc_building_stat))
  (`/Game/BuildingSystem/Blueprints/Classes/BpC_Master_StateManager.ModifyStat` _bpc_building_stat "NewEnumerator2" (`KismetMathLibrary.FCeil` (/ (`KismetMathLibrary.Conv_IntToDouble` _out) (`KismetMathLibrary.Conv_IntToDouble` (`KismetMathLibrary.FFloor` (/ (`self.BuildingTime`) (`self.InterVal`)))))))
  (if (== (`/Game/BuildingSystem/Blueprints/Classes/BpC_Master_StateManager.GetStat` _bpc_building_stat "NewEnumerator2") _out)
    (`self.OnBuildingEnd`)))

(event `OnEnterPlayerSight`
  (set `self.InPlayerSight?` true)
  (if (`self.Built?`)
    (`/Game/BuildingSystem/Widgets/W_BuildingHealthBar.UpdateHealth` (`self.HealthBarRef`) (`/Game/BuildingSystem/Blueprints/Classes/BpC_Master_StateManager.GetStat` (`self.BpC_Building_Stat`) "NewEnumerator2"))
    (`SceneComponent.SetVisibility` (`self.HealthBar`) true false)))

(event `OnBuildingEnd`
  (if (`KismetSystemLibrary.K2_IsValidTimerHandle` (`self.BuildingTimerHandle`))
    (`KismetSystemLibrary.K2_ClearAndInvalidateTimerHandle` (`self.BuildingTimerHandle`))
    (`/Game/BuildingSystem/Widgets/W_BuildingHealthBar.SetState` (`self.HealthBarRef`) "NewEnumerator1")))

(event `OnLeavePlayerSight`
  (set `self.InPlayerSight?` false)
  (if (`self.Built?`)
    (`SceneComponent.SetVisibility` (`self.HealthBar`) false false)))

(event `self.Box.OnComponentBeginOverlap`
  (params (OverlappedComponent :type "PrimitiveComponent Object Reference") (OtherActor :type "Actor Object Reference") (OtherComp :type "PrimitiveComponent Object Reference") (OtherBodyIndex :type Integer) (bFromSweep :type Boolean) (SweepResult :type "HitResult Structure (by ref)"))
  (if (!= OtherActor self)
    (cast `StaticMeshComponent` OtherComp)
    (bind _asbp_master_building (cast `/Game/BuildingSystem/Blueprints/Classes/BuildingClass/Bp_Master_Building` OtherActor))
    (if (`/Game/BuildingSystem/Blueprints/Classes/BuildingClass/Bp_Master_Building.Built?` _asbp_master_building)
      (`BlueprintSetLibrary.Set_Add` (`self.OverLappingBuildings`) _asbp_master_building)
      (if (not (`self.OverLapping?`))
        (`self.OnOverLappingBegin`)))))

(event `self.Box.OnComponentEndOverlap`
  (params (OverlappedComponent :type "PrimitiveComponent Object Reference") (OtherActor :type "Actor Object Reference") (OtherComp :type "PrimitiveComponent Object Reference") (OtherBodyIndex :type Integer))
  (bind _overlappingbuildings (`self.OverLappingBuildings`))
  (if (!= OtherActor self)
    (cast `StaticMeshComponent` OtherComp)
    (bind _asbp_master_building (cast `/Game/BuildingSystem/Blueprints/Classes/BuildingClass/Bp_Master_Building` OtherActor))
    (if (`BlueprintSetLibrary.Set_Contains` (`self.OverLappingBuildings`) _asbp_master_building)
      (`BlueprintSetLibrary.Set_Remove` _overlappingbuildings _asbp_master_building)
      (bind _result (`BlueprintSetLibrary.Set_ToArray` _overlappingbuildings))
      (if (<= (`KismetArrayLibrary.Array_Length` _result) 0)
        (`self.OnOverlappingEnd`)))))

(event `OnOverLappingBegin`
  (set `self.OverLapping?` true)
  (`SceneComponent.SetVisibility` (`self.BuildWidget`) false false)
  (`SceneComponent.SetVisibility` (`self.BuildingMesh`) false false))

(event `OnOverlappingEnd`
  (set `self.OverLapping?` false)
  (`SceneComponent.SetVisibility` (`self.BuildWidget`) true false)
  (`SceneComponent.SetVisibility` (`self.BuildingMesh`) true false))

(fn `ChangeBuildingDirection`
  (locals (`90` :type "Float (double-precision)" :default 90.0))
  (`self.K2_SetActorRotation` self (`KismetMathLibrary.MakeRotator` (.roll (`self.K2_GetActorRotation` self)) (.pitch (`self.K2_GetActorRotation` self)) (+ (.yaw (`self.K2_GetActorRotation` self)) (`local.90`))) false))

(fn `ChangeResource`
  (params (NewResource :type "/Game/BuildingSystem/Blueprints/Classes/ResourceClass/Bp_Master_Resource Class Reference"))
  (bind _resource (`self.Resource`))
  (if (and (`KismetSystemLibrary.IsValidClass` NewResource) (!= NewResource (`self.Resource`)))
    (set `self.Resource` NewResource)
    (`self.UpdateGhostMaterial`)
    (`/Game/BuildingSystem/Widgets/W_BuildingWidget.Update` (`self.BuildWidgetReference`) (`BlueprintMapLibrary.Map_Find` (`self.ResourceVersions`) _resource) _resource)
    (return)
    (else
      (return))))

(fn `UpdateGhostMaterial`
  (`MaterialInstanceDynamic.SetVectorParameterValue` (`self.DynamicMaterial`) "Color" (`.GhostBuildingColor_8_A709DDB14B98E6C39D8389B8B8C81541` (break `/Game/BuildingSystem/Blueprints/Structures/s_ResourceData` (defaults `Object` (`self.Resource`)))))
  (return))

(fn `UserConstructionScript`)