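; FPSCharacter is a player character Blueprint that toggles between a side-view Idle state and a first-person Fight state.
; BeginPlay adds the combat Enhanced Input context, starts in Idle and picks up a rifle; Destroyed removes the context.
; The Aim input flips the state, and SwitchSight swaps active cameras and owner visibility of the two meshes.
; Entering Fight also snaps any equipped gun to the FPS mesh's hand socket.
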(event `EnhancedInput|/Game/Blueprints/Input/Actions/Aim`
  (params (ActionValue :type Boolean) (ElapsedSeconds :type "Float (single-precision)") (TriggeredSeconds :type "Float (single-precision)"))
  (:`Triggered`
    (`KismetSystemLibrary.PrintString` "Hello")
    (switch `CharacterState` (`self.State`)
      (:`Fight`
        (bind _output_get (set `self.State` "Idle"))
        (`self.SwitchSight` _output_get))
      (:`Idle`
        (bind _output_get_2 (set `self.State` "Fight"))
        (`self.SwitchSight` _output_get_2)))))

(event `self.ReceiveBeginPlay`
  (`parent.ReceiveBeginPlay`)
  (`|ExecutionSequence`
    (:`then_0`
      (`EnhancedInputSubsystemInterface.AddMappingContext` (pcsubsystem `EnhancedInputLocalPlayerSubsystem` (`GameplayStatics.GetPlayerController` 0)) "/Game/Blueprints/Input/EI_Combat.EI_Combat" 0)
      (bind _output_get (set `self.State` "Idle"))
      (`self.SwitchSight` _output_get))
    (:`then_1`
      (`self.PickUpGun` "/Game/Blueprints/Guns/Gun_Rifle.Gun_Rifle_C"))))

(event `self.ReceiveDestroyed`
  (`EnhancedInputSubsystemInterface.RemoveMappingContext` (pcsubsystem `EnhancedInputLocalPlayerSubsystem` (`GameplayStatics.GetPlayerController` 0)) "/Game/Blueprints/Input/EI_Combat.EI_Combat"))

(fn `SwitchSight`
  (params (State :type "CharacterState Enum" :default "Fight"))
  (bind _equippedgun (`self.EquippedGun`))
  (switch `CharacterState` State
    (:`Fight`
      (`ActorComponent.Activate` (`self.FPSCameraComponent`) false)
      (`ActorComponent.Deactivate` (`self.SideViewCameraComponent`))
      (`PrimitiveComponent.SetOwnerNoSee` (`self.FPSMesh`) false)
      (`PrimitiveComponent.SetOwnerNoSee` (`self.Mesh`) true)
      (`/Engine/EditorBlueprintResources/StandardMacros.IsValid` _equippedgun
        (:`Is Valid`
          (`self.K2_AttachToComponent` _equippedgun (`self.FPSMesh`) "socket_hand_r" "SnapToTarget" "SnapToTarget" "KeepRelative" true))))
    (:`Idle`
      (`ActorComponent.Activate` (`self.SideViewCameraComponent`) false)
      (`ActorComponent.Deactivate` (`self.FPSCameraComponent`))
      (`PrimitiveComponent.SetOwnerNoSee` (`self.FPSMesh`) true)
      (`PrimitiveComponent.SetOwnerNoSee` (`self.Mesh`) false))))

(fn `UserConstructionScript`)