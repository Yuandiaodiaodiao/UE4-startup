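; Light_Blueprint is an actor that attaches to a Gun_Basic weapon as a child actor, apparently as a light attachment.
; Its construction script casts the parent actor to Gun_Basic and stores it as the equipped gun.
; Logic scaling the gun's RPM and range by multiplier variables is present but disconnected, so it never runs.
; The event graph holds only disabled default events.
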(fn `UserConstructionScript`
  ;[1 1 1] 检测所装备的枪械
  (bind _asgun_basic (cast `/Game/Blueprints/Guns/Gun_Basic` (`self.GetParentActor`)))
  (set `self.GunWhichEquiped` _asgun_basic))