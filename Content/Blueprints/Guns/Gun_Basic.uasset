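; Basic hitscan gun Blueprint that fires from its muzzle along the forward vector up to its range.
; Shoot2 fires only when a time-based cooldown derived from RPM allows it, then calls Shoot.
; Shoot plays effects and sound, line-traces on Visibility with a debug line, and spawns an explosion and applies damage on hit.
; Construction fills RoundRemaining from Magazine, but firing neither checks nor decrements it.
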(event `self.shoot2`
  (bind _muzzle (`self.Muzzle`))
  (bind _returnvalue (`SceneComponent.K2_GetComponentLocation` _muzzle))
  (bind _canshoot (`self.ifCanShootThenShoot`))
  (if _canshoot
    (`self.shoot` _returnvalue (+ _returnvalue (* (`SceneComponent.GetForwardVector` _muzzle) (`self.Range`))))))

(event `self.shoot`
  (params (StartLocation :type "Vector Structure") (EndLocation :type "Vector Structure"))
  (bind _output_get (set `self.NewVar_3` StartLocation))
  (bind _output_get_2 (set `self.NewVar_4` EndLocation))
  (`GameplayStatics.SpawnEmitterAtLocation` (`self.NewVar_1`) _output_get_2)
  (`GameplayStatics.PlaySoundAtLocation` (`self.GunShotSoundEffect`) _output_get (struct) 1.0 1.0 0.0 null null null)
  (bind (_outhit _returnvalue) (`KismetSystemLibrary.LineTraceSingle` :`Start` _output_get :`End` _output_get_2 :`TraceChannel` "TraceTypeQuery1" :`DrawDebugType` "ForDuration" :`TraceColor` (struct :`R` 1000.0 :`A` 1.0) :`DrawTime` 0.2))
  (if _returnvalue
    (bind (_bblockinghit _binitialoverlap _time _distance _location _impactpoint _normal _impactnormal _physmat _hitactor) (`GameplayStatics.BreakHitResult` _outhit))
    (`GameplayStatics.SpawnEmitterAtLocation` "/Game/StarterContent/Particles/P_Explosion.P_Explosion" _location)
    (`GameplayStatics.ApplyDamage` _hitactor (`self.Damage`))))

(fn `ifCanShootThenShoot`
  (returns (canShoot :type Boolean))
  (if (>= (`GameplayStatics.GetTimeSeconds`) (`self.CanShootTime`))
    (set `self.CanShootTime` (+ (`GameplayStatics.GetTimeSeconds`) (/ 60.0 (`self.RPM`))))
    (return true)
    (else
      (return false))))

(fn `UserConstructionScript`
  (set `self.RoundRemaining` (`self.Magazine`)))