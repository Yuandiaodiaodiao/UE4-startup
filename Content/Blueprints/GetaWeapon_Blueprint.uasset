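; Weapon pickup actor that displays a spinning gun and hands it to the player on touch.
; On BeginPlay it spawns a GunType actor at its root transform and spins it in yaw with the Roller timeline.
; When the player pawn overlaps the Box, it calls PickUpGun on GroundCharacter with that class, then destroys itself and the display gun.
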(event `self.ReceiveBeginPlay`
  (bind _returnvalue (`|SpawnActorFromClass` (`self.GunType`) (`SceneComponent.K2_GetComponentToWorld` (`self.DefaultSceneRoot`)) "AlwaysSpawn" "OverrideRootScale" null null))
  (bind _output_get (set `self.GunBeShowed` _returnvalue))
  (bind (_direction _360) (`Timeline|Roller`)
    (:`Update`
      (`SceneComponent.K2_SetRelativeRotation` (`Actor.RootComponent` _output_get) (`KismetMathLibrary.MakeRotator` 0.0 0.0 _360) false false))))

(event `self.Box.OnComponentBeginOverlap`
  (params (OverlappedComponent :type "PrimitiveComponent Object Reference") (OtherActor :type "Actor Object Reference") (OtherComp :type "PrimitiveComponent Object Reference") (OtherBodyIndex :type Integer) (bFromSweep :type Boolean) (SweepResult :type "HitResult Structure (by ref)"))
  (if (== OtherActor (`GameplayStatics.GetPlayerPawn` 0))
    (bind _asground_character (cast `/Game/SideScrollerCPP/Blueprints/GroundCharacter` OtherActor))
    (`/Game/SideScrollerCPP/Blueprints/GroundCharacter.PickUpGun` _asground_character (`self.GunType`))
    (`self.Gun is Picked` false)
    (`self.K2_DestroyActor` (`self.GunBeShowed`))))

(fn `Gun is Picked`
  (params (NewParam :type Boolean))
  (`self.K2_DestroyActor`))

(fn `Spawn a Gun`)

(fn `UserConstructionScript`)