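; Rocket projectile actor that damages whatever it hits, then removes itself.
; On begin play it shrinks its sphere component to a small scale.
; The first hit activates a particle system, applies point damage to the other actor along the hit normal and prints the result.
; A Hurted flag blocks repeat damage, and a short delay precedes destroying the actor.
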(event `self.ReceiveHit`
  (params (MyComp :type "PrimitiveComponent Object Reference") (Other :type "Actor Object Reference") (OtherComp :type "PrimitiveComponent Object Reference") (bSelfMoved :type Boolean) (HitLocation :type "Vector Structure") (HitNormal :type "Vector Structure") (NormalImpulse :type "Vector Structure") (Hit :type "HitResult Structure (by ref)"))
  (if (not (`self.Hurted`))
    (`ActorComponent.Activate` (`self.ParticleSystem`) false)
    (bind _returnvalue (`GameplayStatics.ApplyPointDamage` Other 100.0 HitNormal Hit null self "/Script/Engine.DamageType"))
    (`KismetSystemLibrary.PrintString` (`KismetStringLibrary.Conv_DoubleToString` _returnvalue))
    (set `self.Hurted` true)
    (`KismetSystemLibrary.Delay` 0.2)
    (`self.K2_DestroyActor`)))

(event `self.ReceiveBeginPlay`
  (`SceneComponent.SetWorldScale3D` (`self.Sphere`) (0.2 0.2 0.2)))

(fn `UserConstructionScript`)