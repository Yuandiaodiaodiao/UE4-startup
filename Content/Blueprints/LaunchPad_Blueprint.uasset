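; Launch pad Blueprint that propels the player character when it touches the pad's box trigger.
; On overlap it accepts only the first player's pawn and casts it to Character.
; It then plays its audio component and a 2D sound, activates a particle system, and launches the character by SetSpeed.
; Both override flags are off, so the launch velocity adds to the character's current velocity.
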(event `self.Box.OnComponentBeginOverlap`
  (params (OverlappedComponent :type "PrimitiveComponent Object Reference") (OtherActor :type "Actor Object Reference") (OtherComp :type "PrimitiveComponent Object Reference") (OtherBodyIndex :type Integer) (bFromSweep :type Boolean) (SweepResult :type "HitResult Structure (by ref)"))
  (bind _returnvalue (`GameplayStatics.GetPlayerPawn` 0))
  (if (== OtherActor _returnvalue)
    (bind `_as角色` (cast `Character` _returnvalue))
    (`AudioComponent.Play` (`self.Audio`) 0.0)
    (`ActorComponent.Activate` (`self.ParticleSystem`) false)
    (`GameplayStatics.PlaySound2D` null 1.0 1.0 0.0 null null)
    (`Character.LaunchCharacter` `_as角色` (`self.setSpeed`) false false)))

(fn `UserConstructionScript`)