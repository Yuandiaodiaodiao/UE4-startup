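; BpC_Building_Stat is a building component that holds the stats of a building, such as health, in a States map of min, current and max values.
; InitializeManager sets the Building reference after a validity check, then runs SetUpStats.
; SetMaxStatValue changes the maximum of any existing stat except the health enum entry, clamps its current value and optionally calls UpdateStat.
; UpdateStat is empty, with its health bar refresh logic left disconnected.
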(event `InitializeManager`
  (`/Engine/EditorBlueprintResources/StandardMacros.IsValid` null
    (:`Is Valid`
      (set `self.Building` null)
      (`self.SetUpStats`))))

(fn `GetMaxHealth`
  (returns (Out :type Integer))
  (return (`.MaxValue_8_47BC8CE94C6ABB145A7CD1A83BBD47C3` (break `/Game/Blueprints/BuildingSystem/Blueprints/Structures/s_StatValue` (`.Stat Value` (`self.GetStat` "NewEnumerator0"))))))

(fn `SetMaxStatValue`
  (params (Stat :type "/Game/Blueprints/BuildingSystem/Blueprints/Enums/e_Stats Enum" :default "NewEnumerator0") (NewValue :type Integer) (`Update?` :type Boolean))
  (locals (LocalStat :type "/Game/Blueprints/BuildingSystem/Blueprints/Enums/e_Stats Enum" :default "NewEnumerator0") (LocalValue :type Integer) (LocalUpdate :type Boolean))
  (bind _localvalue (`local.LocalValue`))
  (bind (_currentvalue _stat_value) (`self.GetStat` (`local.LocalStat`)))
  (bind _minvalue (break `/Game/Blueprints/BuildingSystem/Blueprints/Structures/s_StatValue` _stat_value))
  (set `local.LocalStat` Stat)
  (set `local.LocalValue` NewValue)
  (set `local.LocalUpdate` `Update?`)
  (bind _keys (`BlueprintMapLibrary.Map_Keys` (`self.States`)))
  (if (and (`KismetArrayLibrary.Array_Contains` _keys (`local.LocalStat`)) (`|EnumInequality` (`local.LocalStat`) "NewEnumerator0"))
    (`BlueprintMapLibrary.Map_Add` (`self.States`) (`local.LocalStat`) (make `/Game/Blueprints/BuildingSystem/Blueprints/Structures/s_StatValue` _minvalue (`KismetMathLibrary.Clamp` _currentvalue _minvalue _localvalue) _localvalue))
    (if (`local.LocalUpdate`)
      (`self.UpdateStat` (`local.LocalStat`))
      (return)
      (else
        (return)))
    (else
      (return))))

(fn `UpdateStat`
  (params (Stat :type "/Game/Blueprints/BuildingSystem/Blueprints/Enums/e_Stats Enum" :default "NewEnumerator0")))