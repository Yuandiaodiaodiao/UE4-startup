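; Util is a helper Blueprint that converts the mouse cursor position into world space for a given character.
; MouseWorldLocation casts the character's controller to PlayerController, deprojects the mouse position, and returns the world location and direction.
; The EventGraph holds only unconnected copies of this logic that get the character through GetInstance and never run.
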(fn `MouseWorldLocation`
  (params (Character :type "ACharacter Object Reference"))
  (returns (WorldLocation :type "Vector Structure") (WorldDirection :type "Vector Structure"))
  (bind `_as玩家控制器` (cast `PlayerController` (`Pawn.GetController` Character)))
  (bind (_worldlocation _worlddirection) (`PlayerController.DeprojectMousePositionToWorld` `_as玩家控制器`))
  (bind _output_get (set `self.NewVar_0` _worldlocation))
  (bind _output_get_2 (set `self.NewVar_1` _worlddirection))
  (return _output_get _output_get_2))