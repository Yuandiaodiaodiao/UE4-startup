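; BeamActor is an actor that shoots a particle beam which grows steadily along its forward direction.
; Every Tick calls OnShoot, which advances BeamHead at constant speed along the Beam's forward vector, scaled by delta time.
; It then sets the beam emitter's target point one further step ahead of the moved head.
; BeginPlay only prints a placeholder greeting after a short delay, with no effect on the beam.
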(event `self.ReceiveBeginPlay`
  (`KismetSystemLibrary.Delay` 2.0)
  (`KismetSystemLibrary.PrintText` "Hello"))

(event `OnShoot`
  (params (DeltaTime :type "Float (double-precision)"))
  (bind _returnvalue (+ (`SceneComponent.K2_GetComponentLocation` (`self.BeamHead`)) (* (* (`SceneComponent.GetForwardVector` (`self.Beam`)) 600.0) DeltaTime)))
  (`SceneComponent.K2_SetWorldLocation` (`self.BeamHead`) _returnvalue false false)
  (`ParticleSystemComponent.SetBeamTargetPoint` (`self.Beam`) 0 _returnvalue 0))

(event `self.ReceiveTick`
  (params (DeltaSeconds :type "Float (single-precision)"))
  (`self.OnShoot` DeltaSeconds))

(fn `UserConstructionScript`)