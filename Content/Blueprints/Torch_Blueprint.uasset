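; Torch actor that the player can put out and relight with the Use input while nearby.
; Box overlap enables input and opens a Gate, and end overlap disables input and closes it.
; A Use press through the open Gate checks that the overlapping actor is the player pawn, then a FlipFlop toggles the point light intensity and particle system, switching off first.
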(event `InputAction|Use`
  (params (Key :type "Key Structure"))
  (bind _pointlight (`self.PointLight`))
  (:`Pressed`
    (`/Engine/EditorBlueprintResources/StandardMacros.Gate` true :!label _label
      (:`Exit`
        (if (== (stale `self.Box.OnComponentBeginOverlap` OtherActor) (`GameplayStatics.GetPlayerPawn` 0))
          (`/Engine/EditorBlueprintResources/StandardMacros.FlipFlop`
            (:`A`
              (`LightComponent.SetIntensity` _pointlight 0.0)
              (`ActorComponent.Deactivate` (`self.ParticleSystem`)))
            (:`B`
              (`LightComponent.SetIntensity` _pointlight 45000.0)
              (`ActorComponent.Activate` (`self.ParticleSystem`) false))))))))

(event `self.Box.OnComponentBeginOverlap`
  (params (OverlappedComponent :type "PrimitiveComponent Object Reference") (OtherActor :type "Actor Object Reference") (OtherComp :type "PrimitiveComponent Object Reference") (OtherBodyIndex :type Integer) (bFromSweep :type Boolean) (SweepResult :type "HitResult Structure (by ref)"))
  (`self.EnableInput` (`GameplayStatics.GetPlayerController` 0))
  (goto _label :!via `Open`))

(event `self.Box.OnComponentEndOverlap`
  (params (OverlappedComponent :type "PrimitiveComponent Object Reference") (OtherActor :type "Actor Object Reference") (OtherComp :type "PrimitiveComponent Object Reference") (OtherBodyIndex :type Integer))
  (`self.DisableInput` (`GameplayStatics.GetPlayerController` 0))
  (goto _label :!via `Close`))

(fn `UserConstructionScript`)